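; ToggleButtonBP is a hand-gameplay button prop that switches its mesh between an on and an off material when pressed.
; It extends a parent button, running the parent's BeginPlay and then binding a handler to the OnButtonPress dispatcher.
; Each press compares the current slot 0 material with OffMaterial to choose the next one, so the material itself serves as the toggle state.
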(event Custom|OnButtonPressed
  (bind _mesh (Variables|Character|GetMesh))
  (bind _offmaterial (Variables|Default|GetOffMaterial))
  (Rendering|Material|SetMaterial _mesh 0 (select (== _offmaterial (Rendering|Material|GetMaterial _mesh 0)) (Variables|Default|GetOnMaterial) _offmaterial)))

(event EventBeginPlay
  (|CallParentFunction)
  (EventDispatchers|BindEventtoOnButtonPress (EventDispatchers|CreateEvent :!event Custom|OnButtonPressed)))

(fn ConstructionScript
  (|CallParentFunction))