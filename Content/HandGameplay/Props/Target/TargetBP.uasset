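; Target prop that spins when hit and plays audio whose volume follows the spin.
; OnHit adds a velocity-change angular impulse on Y, scaled by SpinSpeed and frame delta time, and enables actor tick.
; Tick maps physics angular speed to the volume multiplier, then disables itself once that value is near zero, so it only runs while the target is moving.
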(event Custom|OnHit
  (Class|PrimitiveComponent|AddAngularImpulseinDegrees (Math|Vector|MakeVector 0.0 (* (Utilities|Time|GetWorldDeltaSeconds) (Variables|Default|GetSpinSpeed)) 0.0) "None" true)
  (Actor|Tick|SetActorTickEnabled true))

(event EventTick
  (params (DeltaSeconds :type Float%20%28single-precision%29))
  (bind _returnvalue (Physics|GetPhysicsAngularVelocityinDegrees "None"))
  (bind _returnvalue_2 (Math|Vector|VectorLength _returnvalue))
  (bind _returnvalue_3 (Math|Float|MapRangeClamped _returnvalue_2 0.0 3.6e+02 0.0 1.0))
  (Audio|Components|Audio|SetVolumeMultiplier _returnvalue_3 :!class /Script/Engine.AudioComponent)
  (if (Math|Float|NearlyEqual(Float) _returnvalue_3 0.0 0.001)
    (Actor|Tick|SetActorTickEnabled false)))

(fn ConstructionScript)