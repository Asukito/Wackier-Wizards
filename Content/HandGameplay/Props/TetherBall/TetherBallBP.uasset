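; TetherBallBP is a tetherball prop with a base mesh, cable and ball that plays impact sounds when hit.
; On BeginPlay it sets the cable to tick post-physics and attaches a spawn particle effect to the base.
; Ball hits play a concurrency-limited sound at the impact point.
; Clamped range mappings scale volume by impulse magnitude, with a threshold select that effectively mutes weak hits.
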(event OnComponentHit(Ball)
  (params (HitComponent :type Primitive%20Component%20Object%20Reference) (OtherActor :type Actor%20Object%20Reference) (OtherComp :type Primitive%20Component%20Object%20Reference) (NormalImpulse :type Vector :default "0, 0, 0") (Hit :type Hit%20Result%20Structure%20%28by%20ref%29))
  (bind _returnvalue (Math|Vector|VectorLength NormalImpulse))
  (Audio|PlaySoundatLocation "/Game/HandGameplay/Props/TetherBall/SFX/TetherBallHit.TetherBallHit" (.impactpoint Hit) "0, 0, 0" (Math|Float|SelectFloat (Math|Float|MapRangeClamped _returnvalue 1e+02 3e+02 0.0 0.5) (Math|Float|MapRangeClamped _returnvalue 3e+02 1e+03 0.5 1.25) (< _returnvalue 1e+02)) 1.0 0.0 0 "/Game/HandGameplay/Props/TetherBall/SFX/TetherBallSoundConcurrency.TetherBallSoundConcurrency" self))

(event EventBeginPlay
  (Components|Tick|SetTickGroup (Variables|Default|GetCable) "TG_PostPhysics")
  (Effects|SpawnEmitterAttached "/Game/HandGameplay/Props/TetherBall/VFX/spawn_tetherballBase_ps.spawn_tetherballBase_ps" (Variables|Default|Gettether_ball_base_sm) "None"))

(fn ConstructionScript)