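; Player character Blueprint that restores saved spells and hosts the spell menus.
; On BeginPlay it reads saved spell IDs from the player data subsystem and passes them back to set the spells.
; Hard-bound C and V keys use FlipFlops to toggle newly created Grimoire and Quick Select widgets, switching input mode and cursor visibility.
; Closing either menu refreshes the spell list component and removes the widget.
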(event EventBeginPlay
  (bind _returnvalue (Subsystems|GetBPPlayerDataSubsystem))
  (bind _returnvalue_2 (Class|PlayerDataSubsystem|GetSavedSpellIDs _returnvalue))
  (Class|PlayerDataSubsystem|SetSpells _returnvalue _returnvalue_2))

(event Input|KeyboardEvents|C
  (params (Key :type Key%20Structure :default "None"))
  (bind _returnvalue (Game|GetPlayerController 0))
  (:Pressed
    (Utilities|FlowControl|FlipFlop
      (:A
        (Input|SetInputModeGameandUI _returnvalue 0 "DoNotLock" false false)
        (Variables|/Script/Engine.PlayerController|SetbShowMouseCursor _returnvalue true)
        (bind _returnvalue_2 (UserInterface|CreateWidget "/Game/1WWDEV/Ben-H/Blueprints/UI/W_GrimoireWidget.W_GrimoireWidget_C"))
        (UserInterface|Viewport|AddtoViewport _returnvalue_2 0))
      (:B
        (Input|SetInputModeGameOnly _returnvalue false)
        (Variables|/Script/Engine.PlayerController|SetbShowMouseCursor _returnvalue false)
        (Default|SetSpells (Variables|Default|GetAC_Spell_List))
        (Widget|RemovefromParent _returnvalue_2)))))

(event Input|KeyboardEvents|V
  (params (Key :type Key%20Structure :default "None"))
  (bind _returnvalue (Game|GetPlayerController 0))
  (:Pressed
    (Utilities|FlowControl|FlipFlop
      (:A
        (Input|SetInputModeGameandUI _returnvalue 0 "DoNotLock" false false)
        (Variables|/Script/Engine.PlayerController|SetbShowMouseCursor _returnvalue true)
        (bind _returnvalue_2 (UserInterface|CreateWidget "/Game/DEVS/Ben-S/UI/SpellUI/W_QuickSelect.W_QuickSelect_C"))
        (UserInterface|Viewport|AddtoViewport _returnvalue_2 0))
      (:B
        (Input|SetInputModeGameOnly _returnvalue false)
        (Variables|/Script/Engine.PlayerController|SetbShowMouseCursor _returnvalue false)
        (Default|SetSpells (Variables|Default|GetAC_Spell_List))
        (Widget|RemovefromParent _returnvalue_2)))))

(fn ConstructionScript)