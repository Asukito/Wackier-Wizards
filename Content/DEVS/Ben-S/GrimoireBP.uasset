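; GrimoireBP is a VR grimoire prop that shows its UI when the BP_VRTest character enters its trigger box.
; Begin overlap triggers a PlayAnimation call on the rigged book, creates a fresh W_GrimoireWidget for the book's widget component, and disables collision on the character's own widget.
; End overlap plays AS_Grimoire1, clears the book's widget, and restores the character widget's UI collision profile.
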(event OnComponentBeginOverlap(Box)
  (params (OverlappedComponent :type Primitive%20Component%20Object%20Reference) (OtherActor :type Actor%20Object%20Reference) (OtherComp :type Primitive%20Component%20Object%20Reference) (OtherBodyIndex :type Integer) (bFromSweep :type Boolean) (SweepResult :type Hit%20Result%20Structure%20%28by%20ref%29))
  (bind _asbp_vrtest (Utilities|Casting|CastToBP_VRTest OtherActor))
  (Variables|Default|SetVRCharacter _asbp_vrtest)
  (Components|Animation|PlayAnimation (Variables|Default|GetGrimoire_rigged04) 0 false)
  (bind _returnvalue (UserInterface|CreateWidget "/Game/1WWDEV/Ben-H/Blueprints/UI/Grimoire/W_GrimoireWidget.W_GrimoireWidget_C"))
  (bind _output_get (Variables|Default|SetGrimoire _returnvalue))
  (UserInterface|SetWidget (Variables|Default|GetWidget) _output_get)
  (Collision|SetCollisionProfileName (Variables|/Script/Wackier_Wizards.VRCharacter|GetwidgetComponent (Variables|Default|GetVRCharacter)) "NoCollision" false :!class /Script/Engine.PrimitiveComponent))

(event OnComponentEndOverlap(Box)
  (params (OverlappedComponent :type Primitive%20Component%20Object%20Reference) (OtherActor :type Actor%20Object%20Reference) (OtherComp :type Primitive%20Component%20Object%20Reference) (OtherBodyIndex :type Integer))
  (bind _asbp_vrtest (Utilities|Casting|CastToBP_VRTest OtherActor))
  (Components|Animation|PlayAnimation (Variables|Default|GetGrimoire_rigged04) "/Game/DEVS/Ben-S/AS_Grimoire1.AS_Grimoire1" false)
  (UserInterface|SetWidget (Variables|Default|GetWidget) 0)
  (Collision|SetCollisionProfileName (Variables|/Script/Wackier_Wizards.VRCharacter|GetwidgetComponent _asbp_vrtest) "UI" false :!class /Script/Engine.PrimitiveComponent))

(fn ConstructionScript)