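; VR character Blueprint with hand-tracking parts for each hand: poseable meshes, pose recognizers, selectors, grabbing and throw assist.
; Its graphs are effectively inert: events are empty, and the tracking-origin, logging and per-hand component wiring nodes are all disconnected.
; LogHand is a debug helper for recording grab poses, dumping a recognizer's encoded hand pose and interactables near that hand's selector to the output log.
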(event EventBeginPlay)

(event Collision|EventActorBeginOverlap
  (params (OtherActor :type Actor%20Object%20Reference)))

(event EventTick
  (params (DeltaSeconds :type Float%20%28single-precision%29)))

(event Input|MouseEvents|ThumbMouseButton
  (params (Key :type Key%20Structure :default "None"))
  ;[1 1 1 1 12] Dumping hand poses and gesture state to output window
)

(event Input|MouseEvents|ThumbMouseButton2
  (params (Key :type Key%20Structure :default "None"))
  ;[1 1 1 1 12] Dumping hand poses and gesture state to output window
)

(fn ConstructionScript)